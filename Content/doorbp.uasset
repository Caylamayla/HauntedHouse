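; Interactive door Blueprint that the player swings open and closed with the use action while standing near it.
; On BeginPlay it binds ToggleDoor to the first-person character's OnUseAction event, and Box overlaps with that character set the IsInDoorZone flag.
; When in the zone, a FlipFlop alternately plays and reverses a Timeline that drives the door's relative yaw from a 90-degree offset, with debug prints throughout.
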(event OnComponentBeginOverlap(Box)
  (params (OverlappedComponent :type Primitive%20Component%20Object%20Reference) (OtherActor :type Actor%20Object%20Reference) (OtherComp :type Primitive%20Component%20Object%20Reference) (OtherBodyIndex :type Integer) (bFromSweep :type Boolean) (SweepResult :type Hit%20Result%20Structure%20%28by%20ref%29))
  ;[1 1 1] Player Entered
  (Utilities|Casting|CastToFirstPersonCharacter OtherActor)
  (Development|PrintString "Overlap!")
  (Variables|Default|SetIsInDoorZone true))

(event OnComponentEndOverlap(Box)
  (params (OverlappedComponent :type Primitive%20Component%20Object%20Reference) (OtherActor :type Actor%20Object%20Reference) (OtherComp :type Primitive%20Component%20Object%20Reference) (OtherBodyIndex :type Integer))
  ;[1 1 1] Player Exited
  (Utilities|Casting|CastToFirstPersonCharacter OtherActor)
  (Development|PrintString "End Overlap")
  (Variables|Default|SetIsInDoorZone false))

(event Custom|ToggleDoor
  (if (Variables|Default|GetIsInDoorZone)
    (Development|PrintString "Toggle door! 
")
    (Utilities|FlowControl|FlipFlop
      (:A
        (bind _timeline (Timeline|Timeline_0 Play)
          (:Update
            (Transformation|SetRelativeRotation (Variables|Default|Getdoor) (Math|Rotator|MakeRotator 0.0 0.0 (+ _timeline 9e+01)) false false))))
      (:B
        (Timeline|Timeline_0 Reverse)))))

(event EventBeginPlay
  (bind _asfirst_person_character (Utilities|Casting|CastToFirstPersonCharacter (Game|GetPlayerCharacter 0)))
  (EventDispatchers|BindEventtoOnUseAction _asfirst_person_character (delegate Custom|ToggleDoor)))

(fn ConstructionScript)